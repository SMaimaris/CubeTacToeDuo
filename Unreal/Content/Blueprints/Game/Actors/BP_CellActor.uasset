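; BP_CellActor is a board cell with an owner state, with materials for empty, X and O suggesting tic-tac-toe.
; On BeginPlay it creates a dynamic empty-cell material on its mesh, then tints its HoverColor while the cursor is over an unowned cell.
; Owner changes only call the parent implementation; the Blueprint's material-switching nodes for empty, X and O are disconnected and never run.
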(event `self.ReceiveBeginPlay`
  (`parent.ReceiveBeginPlay`)
  (bind _returnvalue (`PrimitiveComponent.CreateDynamicMaterialInstance` (`self.MeshComponent`) 0 "/Game/Materials/M_CellEmpty.M_CellEmpty" "None"))
  (set `self.EmptyMatDynamic` _returnvalue))

(event `self.OnOwnerChanged`
  (params (NewOwner :type "ECellOwner Enum" :default "None"))
  (`parent.OnOwnerChanged` NewOwner))

(event `self.ReceiveActorBeginCursorOver`
  (`parent.ReceiveActorBeginCursorOver`)
  (switch `ECellOwner` (`self.GetCellOwner`)
    (:`None`
      (`MaterialInstanceDynamic.SetVectorParameterValue` (`self.EmptyMatDynamic`) "HoverColor" (struct :`R` 0.1 :`G` 0.1 :`B` 0.05)))))

(event `self.ReceiveActorEndCursorOver`
  (`parent.ReceiveActorEndCursorOver`)
  (switch `ECellOwner` (`self.GetCellOwner`)
    (:`None`
      (`MaterialInstanceDynamic.SetVectorParameterValue` :`self` (`self.EmptyMatDynamic`) :`ParameterName` "HoverColor"))))

(fn `UserConstructionScript`)