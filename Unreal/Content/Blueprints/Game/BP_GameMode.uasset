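; Game mode for a turn-based X-and-O board game with multiple winnable faces.
; Move, face-win, turn, game-over and turn-timer events all defer to the parent class.
; Only applied moves add behavior, passing the coordinate and player to the first BP_BoardActor found in the level for visuals.
; Unconnected leftover chains hold face-win visuals, HUD refreshes and the game-over screen, so none of those run here.
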(event `self.ReceiveBeginPlay`
  (`parent.ReceiveBeginPlay`))

(event `self.OnMoveApplied`
  (params (Coord :type "CellCoord Structure") (Player :type "ECellOwner Enum" :default "None"))
  (`parent.OnMoveApplied` Coord Player)
  (bind _outactors (`GameplayStatics.GetAllActorsOfClass` "/Game/Blueprints/Game/Actors/BP_BoardActor.BP_BoardActor_C"))
  (`CTTBoardActor.ApplyMoveVisual` (`|GetArrayItem` _outactors) Coord Player))

(event `self.OnFaceWon`
  (params (Face :type "EFaceIndex Enum" :default "Top") (Winner :type "ECellOwner Enum" :default "None"))
  (`parent.OnFaceWon` Face Winner))

(event `self.OnTurnChanged`
  (params (NewPlayer :type "ECellOwner Enum" :default "None"))
  (`parent.OnTurnChanged` NewPlayer))

(event `self.OnGameOver`
  (params (Winner :type "ECellOwner Enum" :default "None") (bIsDraw :type Boolean))
  (`parent.OnGameOver` Winner bIsDraw))

(event `self.OnTurnTimerExpired`
  (params (Player :type "ECellOwner Enum" :default "None"))
  (`parent.OnTurnTimerExpired` Player))

(fn `UserConstructionScript`)